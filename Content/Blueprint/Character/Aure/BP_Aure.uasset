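; BP_Aure is a character Blueprint for Aure that fades overlapping actors, supports motion-warped facing and holds a shock-loop state.
; Box overlaps add actors to FadeActor and send FadeOutMessage to every listed BI_FadeInterface implementer.
; End overlap sends FadeInMessage and removes the actor, only for implementers, so other actors stay listed.
; Events update the MotionWarping FacingTarget location and set the InShockLoop flag.
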(event OnComponentBeginOverlap(Box)
  (params (OverlappedComponent :type Primitive%20Component%20Object%20Reference) (OtherActor :type Actor%20Object%20Reference) (OtherComp :type Primitive%20Component%20Object%20Reference) (OtherBodyIndex :type Integer) (bFromSweep :type Boolean) (SweepResult :type Hit%20Result%20Structure%20%28by%20ref%29))
  (Utilities|Array|AddUnique (Variables|Default|GetFadeActor) OtherActor)
  (for _array_element (Variables|Default|GetFadeActor)
    (if (Utilities|DoesObjectImplementInterface _array_element "/Game/Blueprint/Actor/FadeActor/BI_FadeInterface.BI_FadeInterface_C")
      (Class|BIFadeInterface|FadeOut(Message) _array_element))))

(event OnComponentEndOverlap(Box)
  (params (OverlappedComponent :type Primitive%20Component%20Object%20Reference) (OtherActor :type Actor%20Object%20Reference) (OtherComp :type Primitive%20Component%20Object%20Reference) (OtherBodyIndex :type Integer))
  (Variables|Default|SetFadeActorIndex (Utilities|Array|FindItem (Variables|Default|GetFadeActor) OtherActor))
  (if (Utilities|DoesObjectImplementInterface OtherActor "/Game/Blueprint/Actor/FadeActor/BI_FadeInterface.BI_FadeInterface_C")
    (Class|BIFadeInterface|Fadein(Message) OtherActor)
    (Utilities|Array|RemoveIndex (Variables|Default|GetFadeActor) (Variables|Default|GetFadeActorIndex))))

(event EventBeginPlay)

(event Collision|EventActorBeginOverlap
  (params (OtherActor :type Actor%20Object%20Reference)))

(event EventTick
  (params (DeltaSeconds :type Float%20%28single-precision%29)))

(event EventUpdateFacingTarget
  (params (Target :type Vector%20%28by%20ref%29 :default "0, 0, 0"))
  (Class|MotionWarpingComponent|AddorUpdateWarpTargetfromLocation (Variables|Default|GetMotionWarping) "FacingTarget" Target))

(event EventSetinShockLoop
  (params (bInLoop :type Boolean))
  (Variables|Default|SetInShockLoop bInLoop))

(fn ConstructionScript)