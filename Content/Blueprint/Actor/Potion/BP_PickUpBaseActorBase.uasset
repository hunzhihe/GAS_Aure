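; Base Blueprint for pickup actors, filed under potions, that animates their spawn and idle motion and plays spawn, ground-impact and consumed sounds.
; On BeginPlay a timeline drives scale and height offset from SpawnApex, with a DoOnce impact sound gated by elevation.
; When it finishes, inherited or external functions start rotation and sinusoidal bobbing, while Tick applies the calculated location and rotation.
; Destruction plays the consumed sound; overlap is unimplemented here.
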(event EventBeginPlay
  (bind _calculatedlocation (Variables|Default|GetCalculatedLocation))
  (Audio|PlaySoundatLocation (Variables|Default|GetSpawnSound) (Transformation|GetActorLocation) "0, 0, 0" 1.0 1.0 0.0 0 0 0 0) ; 生成音效
  (bind (_direction _elevation _scale) (Timeline|PickUpElevationTimeline Play)
    (:Update
      ;[0.15 0.15 0.15 0.5] 时间轴更新位置和缩放
      (Transformation|SetActorLocation (Math|Vector|MakeVector (.x _calculatedlocation) (.y _calculatedlocation) (+ (.z _calculatedlocation) (* _elevation (Variables|Default|GetSpawnApex)))) false false)
      (Transformation|SetActorScale3D (Math|Vector|MakeVector _scale _scale _scale))
      (if (> _elevation 0.3)
        (Utilities|FlowControl|DoOnce false
          (:Completed
            (Audio|PlaySoundatLocation (Variables|Default|GetGroundImpactSound) (Transformation|GetActorLocation) "0, 0, 0" 1.0 1.0 0.0 0 0 0 0)))))
    (:Finished
      (Class|AureEffectActor|StartRotation) ; 开始旋转
      (Class|AureEffectActor|StartSinusoidalMovement) ; 开始上下移动
    )))

(event Collision|EventActorBeginOverlap
  (params (OtherActor :type Actor%20Object%20Reference)))

(event EventTick
  (params (DeltaSeconds :type Float%20%28single-precision%29))
  (Transformation|SetActorLocation (Variables|Default|GetCalculatedLocation) false false) ; 更新位置
  (Transformation|SetActorRotation (Variables|Default|GetCalculatedRotation)) ; 更新转向
)

(event EventDestroyed
  (Audio|PlaySoundatLocation (Variables|Default|GetConsumedSound) (Transformation|GetActorLocation) "0, 0, 0" 1.0 1.0 0.0 0 0 0 0) ; 播放拾取音效
)

(fn ConstructionScript)