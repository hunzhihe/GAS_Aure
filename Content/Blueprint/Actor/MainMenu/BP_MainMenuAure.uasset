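; Main menu scene actor that drives the menu's ambient effects and brings up its UI.
; On BeginPlay it plays the menu music, shows WBP_MainMenu with UI-only input and a visible cursor, and caches the Niagara fireball's start position.
; Tick bobs the fireball vertically with a time-based sine around that position and spins the magic circle decal around its roll axis at a configurable rate.
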(event EventBeginPlay
  ;[0.15 0.15 0.15 0.5] 存储火球默认位置
  (Variables|Default|SetFireLocation (Transformation|GetWorldLocation (Variables|Default|GetNiagaraFire)))
  (Audio|PlaySound2D "/Game/Assets/Sounds/Music/Music_MainMenu.Music_MainMenu" 1.0 1.0 0.0 0 0)
  (bind _returnvalue (UserInterface|CreateWidget "/Game/Blueprint/UI/MainMenu/WBP_MainMenu.WBP_MainMenu_C"))
  (UserInterface|Viewport|AddtoViewport _returnvalue 0)
  (Input|SetInputModeUIOnly (Game|GetPlayerController 0) _returnvalue "DoNotLock" false)
  (Variables|/Script/Engine.PlayerController|SetbShowMouseCursor (Game|GetPlayerController 0) true))

(event Collision|EventActorBeginOverlap
  (params (OtherActor :type Actor%20Object%20Reference)))

(event EventTick
  (params (DeltaSeconds :type Float%20%28single-precision%29))
  ;[0.15 0.15 0.15 0.5] 火球上下浮动
  (bind _output_get (Variables|Default|SetTime (+ DeltaSeconds (Variables|Default|GetTime))))
  (Transformation|SetWorldLocation (Variables|Default|GetNiagaraFire) (+ (Variables|Default|GetFireLocation) (Math|Vector|MakeVector 0.0 0.0 (* (Math|Trig|Sin(Radians) _output_get) (Variables|Default|GetAmplitude)))) false false)
  ;[0.15 0.15 0.15 0.5] 魔法阵旋转
  (Transformation|AddLocalRotation (Variables|Default|GetDecal) (Math|Rotator|MakeRotator (* (Variables|Default|GetDelta%20Seconds) (Variables|Default|GetMagicCircleRotationRate)) 0.0 0.0) false false))

(fn ConstructionScript)