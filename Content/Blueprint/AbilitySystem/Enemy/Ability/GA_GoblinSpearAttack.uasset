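; Gameplay ability for the goblin enemy's spear melee attack.
; It turns the avatar toward its combat target through the combat interface, then plays the spear attack montage and waits for the melee montage gameplay event.
; On that event it finds live players within a small sphere at the combat socket, excluding itself, damages each and ends the ability.
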(event Ability|EventActivateAbility
  (bind _returnvalue (Ability|GetAvatarActorfromActorInfo))
  (bind _returnvalue_2 (Ability|GetAvatarActorfromActorInfo))
  (bind _returnvalue_3 (Class|EnemyInterface|GetCombatTarget(Message) _returnvalue))
  (bind _ascombat_interface (Utilities|Casting|CastToCombatInterface _returnvalue)
    (:then
      (Class|CombatInterface|UpdateFacingTarget _ascombat_interface (Transformation|GetActorLocation _returnvalue_3))
      (|PlayMontageandWaitProxy "None" "/Game/Assets/Enemies/Goblin/Animations/Spear/AM_Attack_GoblinSpear.AM_Attack_GoblinSpear" 1.0 "None" true 1.0 0.0 false
        (:then
          (Ability|Tasks|WaitGameplayEvent "(TagName=\"Event.Montage.Attack.Melee\")" 0
            (:EventReceived
              (bind _returnvalue_4 (Class|CombatInterface|GetCombatSocketLocation(Message) _returnvalue_2 (Variables|Default|GetSocketTag)))
              (bind _outoverlappingactors (Class|AuraAbilitySystemLibrary|GetLivePlayersWithinRadius _returnvalue_2 (Utilities|Array|MakeArray _returnvalue_2) 45.0 _returnvalue_4))
              (for _array_element _outoverlappingactors
                (Class|AureDamageGameplayAbility|CauseDamage _array_element))
              (Ability|EndAbility))))))
    (:CastFailed
      (Ability|EndAbility))))

(event Ability|EventOnEndAbility
  (params (bWasCancelled :type Boolean)))