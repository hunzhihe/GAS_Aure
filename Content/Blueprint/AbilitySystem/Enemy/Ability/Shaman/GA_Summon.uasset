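; Shaman enemy gameplay ability that summons a group of random minions at generated spawn points.
; On activation it shuffles the locations, plays a ground Niagara effect at each and starts the summon montage.
; A montage gameplay event triggers staggered spawning of AI-controlled minions facing away from the caster, using a delay loop.
; Each spawn raises the avatar's minion count through an interface message, and a destroy callback lowers it.
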(event Custom|OnDestroyed_事件
  (params (DestroyedActor :type Actor%20Object%20Reference))
  ;[0.15 0.15 0.15 0.5] 召唤位置逐个生成
  (Class|CombatInterface|IncrementMinionCount(Message) (Ability|GetAvatarActorfromActorInfo) -1))

(event Ability|EventActivateAbility
  (bind _returnvalue (Class|AureSummonAbility|GetSpawnLocation))
  (bind _output_get (Variables|Default|SetSpawnLocations _returnvalue))
  (Utilities|Array|Shuffle _output_get) ; 随机生成顺序
  (Utilities|FlowControl|Sequence
    (:then_0
      ;[0.15 0.15 0.15 0.5] 在召唤目标位置生成粒子特效
      (for _array_element (Variables|Default|GetSpawnLocations)
        (Niagara|SpawnSystematLocation "/Game/Assets/Effects/Combat/NS_GroundSummon.NS_GroundSummon" _array_element)))
    (:then_1
      (|PlayMontageandWaitProxy "None" "/Game/Assets/Enemies/Shaman/Animations/AM_Shaman_Summon.AM_Shaman_Summon" 1.0 "None" true 1.0 0.0 false
        (:then
          (Ability|Tasks|WaitGameplayEvent "(TagName=\"CombatSocket.Weapon\")" 0
            (:EventReceived
              ;[0.15 0.15 0.15 0.5] 召唤位置逐个生成
              (Variables|Default|Setindex 0)
              (if (< (Variables|Default|Getindex) (Utilities|Array|Length (Variables|Default|GetSpawnLocations))) :!label _label
                (bind _returnvalue_2 (Game|SpawnActorfromClass (Class|AureSummonAbility|GetRandomMinionClass) (Math|Transform|MakeTransform (+ (Utilities|Array|Get(acopy) (Variables|Default|GetSpawnLocations) (Variables|Default|Getindex)) "0.000000,0.000000,70.000000") (Math|Rotator|FindLookatRotation (Transformation|GetActorLocation (Ability|GetAvatarActorfromActorInfo)) (Utilities|Array|Get(acopy) (Variables|Default|GetSpawnLocations) (Variables|Default|Getindex))) "1.000000,1.000000,1.000000") "AdjustIfPossibleButAlwaysSpawn" "MultiplyWithRoot" 0 0))
                (Pawn|SpawnDefaultController _returnvalue_2)
                (Game|AssignOnDestroyed _returnvalue_2 (delegate Custom|OnDestroyed_事件))
                (Class|CombatInterface|IncrementMinionCount(Message) (Ability|GetAvatarActorfromActorInfo) 1)
                (Math|Integer|IncrementInt (Variables|Default|Getindex)
                  (:%20%20
                    (Utilities|FlowControl|Delay 0.2) ; 时间间隔
                    (goto _label)))))))
        (:OnCompleted
          (Ability|EndAbility :!label _label_2))
        (:OnBlendOut
          (goto _label_2))
        (:OnCancelled
          (goto _label_2))))))

(event Ability|EventOnEndAbility
  (params (bWasCancelled :type Boolean)))