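; Enemy ranged-attack gameplay ability, filed under SlingShot, that fires a projectile at the avatar's combat target.
; On activation it turns the avatar toward the target and plays a random tagged attack montage.
; A one-shot gameplay event matching the montage's socket tag triggers SpawnProjectile from that socket toward the target's current location, then ends the ability.
; No montage completion or interruption path ends it.
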(event Ability|EventActivateAbility
  (bind _returnvalue (Ability|GetAvatarActorfromActorInfo))
  (bind _returnvalue_2 (Ability|GetAvatarActorfromActorInfo))
  ;[0.15 0.15 0.15 0.5] 获取到战斗目标，并朝向目标
  (bind _returnvalue_3 (Class|EnemyInterface|GetCombatTarget(Message) _returnvalue))
  (Class|CombatInterface|UpdateFacingTarget(Message) _returnvalue (Transformation|GetActorLocation _returnvalue_3))
  ;[0.15 0.15 0.15 0.5] 获取到随机的攻击动画播放
  (bind _returnvalue_4 (Class|CombatInterface|GetAttackMontages(Message) (Ability|GetAvatarActorfromActorInfo)))
  (bind _output_get (Variables|Default|SetTaggedMontage (Class|AureDamageGameplayAbility|GetRandomTaggedMontagefromArray _returnvalue_4)))
  ;[0.15 0.15 0.15 0.5] 播放动画，触发事件
  (|PlayMontageandWaitProxy "None" (.Montage (Utilities|Struct|BreakTaggedMontage _output_get)) 1.0 "None" true 1.0 0.0 false
    (:then
      (Ability|Tasks|WaitGameplayEvent (.SocketTag (Utilities|Struct|BreakTaggedMontage _output_get)) 0 true
        (:EventReceived
          ;[0.15 0.15 0.15 0.5] 获取生成子弹的插槽位置，生成子弹
          (Class|CombatInterface|GetCombatSocketLocation(Message) _returnvalue_2 (.SocketTag (Utilities|Struct|BreakTaggedMontage (Variables|Default|GetTaggedMontage))))
          (bind _returnvalue_5 (Class|EnemyInterface|GetCombatTarget(Message) _returnvalue_2))
          (Class|AureProjectSpell|SpawnProjectile (Transformation|GetActorLocation _returnvalue_5) (.SocketTag (Utilities|Struct|BreakTaggedMontage (Variables|Default|GetTaggedMontage))) false 0.0)
          (Ability|EndAbility))))))

(event Ability|EventOnEndAbility
  (params (bWasCancelled :type Boolean)))