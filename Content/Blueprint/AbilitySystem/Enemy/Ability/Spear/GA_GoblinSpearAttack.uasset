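; Gameplay ability for the goblin spear enemy's melee attack.
; On activation it faces the combat target, plays a random tagged attack montage and waits for that montage's socket gameplay event.
; The event triggers a sphere check at the weapon socket that damages non-friendly live players.
; Hit effects and impact sound go through GameplayCues so clients receive them, and the ability ends with the montage.
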(event Ability|EventActivateAbility
  (bind _returnvalue (Ability|GetAvatarActorfromActorInfo))
  (bind _returnvalue_2 (Ability|GetAvatarActorfromActorInfo))
  (Variables|Default|SetHasHitTarget false)
  (bind _returnvalue_3 (Class|EnemyInterface|GetCombatTarget(Message) _returnvalue))
  (bind _ascombat_interface (Utilities|Casting|CastToCombatInterface _returnvalue)
    (:then
      (Class|CombatInterface|UpdateFacingTarget _ascombat_interface (Transformation|GetActorLocation _returnvalue_3))
      ;[0.15 0.15 0.15 0.5] 判断是否设置攻击动画，如果有，则随机使用一组
      (bind _returnvalue_4 (Class|CombatInterface|GetAttackMontages(Message) (Ability|GetAvatarActorfromActorInfo)))
      (bind _output_get (Variables|Default|SetMontageStruct (Class|AureDamageGameplayAbility|GetRandomTaggedMontagefromArray _returnvalue_4)))
      (|PlayMontageandWaitProxy "None" (.Montage (Utilities|Struct|BreakTaggedMontage _output_get)) 1.0 "None" true 1.0 0.0 false
        (:then
          (Ability|Tasks|WaitGameplayEvent (.SocketTag (Utilities|Struct|BreakTaggedMontage _output_get)) 0
            (:EventReceived
              (bind _returnvalue_5 (Class|CombatInterface|GetCombatSocketLocation(Message) _returnvalue_2 (.SocketTag (Utilities|Struct|BreakTaggedMontage (Variables|Default|GetMontageStruct)))))
              (bind _outoverlappingactors (Class|AuraAbilitySystemLibrary|GetLivePlayersWithinRadius _returnvalue_2 (Utilities|Array|MakeArray _returnvalue_2) 45.0 _returnvalue_5))
              (for _array_element _outoverlappingactors
                (if (Class|AuraAbilitySystemLibrary|IsNotFriend _array_element (Ability|GetAvatarActorfromActorInfo))
                  (Class|AureDamageGameplayAbility|CauseDamage _array_element)
                  ;[0.15 0.15 0.15 0.5] GameplayCue,受伤特效
                  (Variables|Default|SetHasHitTarget true)
                  (Variables|Default|SetCombatLocation (Transformation|GetActorLocation _array_element))
                  (Class|GameplayAbility|ExecuteGameplayCuewithParams "(TagName=\"GameplayCue.HitEffect\")" (Ability|GameplayCue|MakeGameplayCueParameters :Location (Variables|Default|GetCombatLocation) :SourceObject _array_element))))
              ;[0.15 0.15 0.15 0.5] 利用GameplayCue,让客户端也可以听见音效
              (if (Variables|Default|GetHasHitTarget) ; 击中敌人播放音效
                (Class|GameplayAbility|ExecuteGameplayCuewithParams "(TagName=\"GameplayCue.ImpactSound\")" (Ability|GameplayCue|MakeGameplayCueParameters :AggregatedSourceTags (GameplayTags|MakeGameplayTagContainerfromTag (.MontageTag (Utilities|Struct|BreakTaggedMontage (Variables|Default|GetMontageStruct)))) :Location (Variables|Default|GetCombatLocation) :EffectCauser (Ability|GetAvatarActorfromActorInfo)))))))
        (:OnCompleted
          (Ability|EndAbility :!label _label))
        (:OnBlendOut
          (goto _label))
        (:OnInterrupted
          (goto _label))
        (:OnCancelled
          (goto _label))))
    (:CastFailed
      (Ability|EndAbility))))

(event Ability|EventOnEndAbility
  (params (bWasCancelled :type Boolean)))