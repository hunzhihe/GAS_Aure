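; Arcane Shards gameplay ability: shows a magic circle, then on input release strikes several ground points around the cursor target.
; A spawned BP_PointCollection supplies randomly rotated points, with count set by ability level up to a cap.
; After the cast montage's gameplay event, a looping timer fires one shard per point via a GameplayCue, applying radial damage.
; Ability end destroys the point actor, clears the timer and hides the circle.
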(event Custom|SpawnShard
  (bind _result (Math|Integer|IncrementInt (Variables|Default|GetIndex))
    (:%20%20
      (if (<= _result (Variables|Default|GetNum%20Points)) ; 若索引大于等于生成数量，则结束技能，停止定时器
        ;[0.15 0.15 0.15 0.5] 获取位置，并播放奥数效果
        (bind _output_get (Variables|Default|SetShardLocation (Transformation|GetWorldLocation (Utilities|Array|Get(acopy) (Variables|Default|GetGroundPoints) (- (Variables|Default|GetIndex) 1)))))
        (GameplayCue|ExecuteGameplayCueOnActor(Burst) (Ability|GetOwningActorfromActorInfo) "(TagName=\"GameplayCue.ArcaneShards\")" (Ability|GameplayCue|MakeGameplayCueParameters :Location _output_get))
        (CallFunction|应用范围伤害)
        (else
          (Ability|EndAbility))))))

(event Custom|激活奥数爆发技能
  (bind _datahandle (|TargetDataUnderMouse) ; 获取鼠标拾取位置
    (:ValidData
      (bind _output_get (Variables|Default|SetImpact%20Point (.ImpactPoint (Collision|BreakHitResult (Ability|TargetData|GetHitResultfromTargetData _datahandle)))))
      ;[0.15 0.15 0.15 0.5] 生成技能攻击位置的随机点，并存储在数组中
      (bind _returnvalue (Game|SpawnActorfromClass "/Game/Blueprint/AbilitySystem/Aure/Ability/ArcaneShards/BP_PointCollection.BP_PointCollection_C" (Math|Transform|MakeTransform _output_get "0, 0, 0" "1.000000,1.000000,1.000000") "AlwaysSpawn" "MultiplyWithRoot" 0 0))
      (bind _output_get_2 (Variables|Default|SetPointCollection _returnvalue))
      (Variables|Default|SetGroundPoints (Class|PointCollection|GetGroundPoints _output_get_2 (Variables|Default|GetImpact%20Point) (Variables|Default|GetNum%20Points) (Math|Random|RandomFloatinRange 0.0 3.6e+02)))
      ;[0.15 0.15 0.15 0.5] 角色朝向，施法动画
      (Class|CombatInterface|UpdateFacingTarget(Message) (Ability|GetAvatarActorfromActorInfo) (Variables|Default|GetImpact%20Point))
      (|PlayMontageandWaitProxy "None" "/Game/Assets/Characters/Aura/Animations/Abilities/AM_Cast_ArcaneShards.AM_Cast_ArcaneShards" 1.0 "None" true 1.0 0.0 false
        (:then
          (Ability|Tasks|WaitGameplayEvent "(TagName=\"Event.Montage.ArcaneShards\")" 0 true
            (:EventReceived
              (CallFunction|生成所有奥数爆发个体))))))))

(event Custom|生成所有奥数爆发个体
  (Variables|Default|SetIndex 0)
  (bind _returnvalue (Utilities|Time|SetTimerbyEvent (delegate Custom|SpawnShard) (Variables|Default|GetShardSpawnTime) true))
  (Variables|Default|SetSpawnTimerHandle _returnvalue)
  (Class|PlayerInterface|HideMagicCircle(Message) (Ability|GetAvatarActorfromActorInfo)) ; 隐藏魔法阵
  (CallFunction|SpawnShard) ; 先调用一次事件，触发后生成一个个体
)

(event Ability|EventActivateAbility
  (Utilities|FlowControl|Sequence
    (:then_0
      (Ability|CommitAbility)
      (Class|PlayerInterface|ShowMagicCircle(Message) (Ability|GetAvatarActorfromActorInfo) 0) ; 技能触发时，显示魔法阵
      (Variables|Default|SetNum%20Points (Math|Integer|Min(Integer) (Variables|Default|GetMaxNumShards) (Ability|GetAbilityLevel))))
    (:then_1
      (Ability|Tasks|WaitInputRelease false
        (:OnRelease
          (CallFunction|激活奥数爆发技能))))))

(event Ability|EventOnEndAbility
  (params (bWasCancelled :type Boolean))
  (bind _pointcollection (Variables|Default|GetPointCollection)
    (:then
      (Actor|DestroyActor _pointcollection)
      (Utilities|Time|ClearandInvalidateTimerbyHandle (Variables|Default|GetSpawnTimerHandle))
      (Class|PlayerInterface|HideMagicCircle(Message) (Ability|GetAvatarActorfromActorInfo)) ; 隐藏魔法阵
    )
    (:else)))

(fn 应用范围伤害
  (bind _returnvalue (Ability|GetAvatarActorfromActorInfo))
  (bind _outoverlappingactors (Class|AuraAbilitySystemLibrary|GetLivePlayersWithinRadius _returnvalue (Utilities|Array|MakeArray _returnvalue) (Variables|Default|GetRadialDamageOuterRadius) (Variables|Default|GetShardLocation)))
  (bind _output_get (Variables|Default|SetOut%20Overlapping%20Actors _outoverlappingactors))
  (for _array_element _output_get
    (Class|AuraAbilitySystemLibrary|ApplyDamageEffect (Class|AureDamageGameplayAbility|MakeDamageEffectParamsfromClassDefaults _array_element (Variables|Default|GetShardLocation) false "0, 0, 0" false "0, 0, 0" true 2e+01))))