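; Fireball projectile for the FireBlast ability that flies outward, homes back to its source actor and explodes on nearing it.
; On the server, two chained timelines lerp it to a forward apex, then back toward ReturnToActor's live location until within ExplodeDistance.
; Boom applies radial GAS damage to live players in range except the owner, with knockback and death impulse pitched 45 degrees, then destroys the fireball.
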(event EventBeginPlay)

(event Collision|EventActorBeginOverlap
  (params (OtherActor :type Actor%20Object%20Reference)))

(event EventStartOutgoingTimeline
  (Networking|SwitchHasAuthority
    (:Authority
      (Variables|Default|SetInitial%20Location (Transformation|GetActorLocation)) ; 初始位置
      (Variables|Default|SetApexLocation (+ (Variables|Default|GetInitial%20Location) (* (Transformation|GetActorForwardVector) (Variables|Default|GetTravelDistance))))
      (bind _outgoingtrack (Timeline|OutgoingTimeline Play) ; 火球向外扩散
        (:Update
          (Transformation|SetActorLocation (Math|Vector|Lerp(Vector) (Variables|Default|GetInitial%20Location) (Variables|Default|GetApexLocation) _outgoingtrack) false false))
        (:Finished
          (bind _returningtrack (Timeline|时间轴 Play) ; 火球返回角色
            (:Update
              (bind _output_get (Variables|Default|SetOwnerLocation (Transformation|GetActorLocation (Variables|Default|GetReturnToActor))))
              (Transformation|SetActorLocation (Math|Vector|Lerp(Vector) (Variables|Default|GetApexLocation) _output_get _returningtrack) false false)
              (if (<= (Math|Vector|Distance(Vector) (Transformation|GetActorLocation) (Variables|Default|GetOwnerLocation)) (Variables|Default|GetExplodeDistance)) ; 返回时，距离玩家一定距离产生爆炸
                (CallFunction|Boom)))))))))

(fn ConstructionScript)

(fn Boom
  (bind _returnvalue (Components|GetOwner))
  (bind _array (Utilities|Array|MakeArray _returnvalue))
  (Class|AuraAbilitySystemLibrary|SetIsRadialDamageEffectParams (Variables|Default|GetExplsionDamage%20Params) true (Variables|Default|GetRadialDamage%20Inner%20Radius) (Variables|Default|GetRadialDamage%20Out%20Radius) (Transformation|GetActorLocation))
  (Utilities|Array|Add _array self)
  (bind _outoverlappingactors (Class|AuraAbilitySystemLibrary|GetLivePlayersWithinRadius (Components|GetOwner) _array (Variables|Default|GetRadialDamage%20Out%20Radius) (Transformation|GetActorLocation)))
  (CallFunction|ApplyGEtoActors _outoverlappingactors)
  (Actor|DestroyActor))

(fn ApplyGEtoActors
  (params (OverlapActors :type Array%20of%20Actor%20Object%20References))
  (bind _output_get (Variables|Default|SetOverlapActors OverlapActors))
  (for _array_element _output_get
    (bind _output_get_2 (Variables|Default|SetOverlapActor _array_element))
    (bind _output_get_3 (Variables|Default|SetTargetAsc (Ability|GetAbilitySystemComponent _output_get_2)))
    (if (Utilities|IsValid _output_get_3)
      (bind _output_get_4 (Variables|Default|SetAttackDirection (- (Transformation|GetActorLocation (Variables|Default|GetOverlapActor)) (Transformation|GetActorLocation)))) ; 获取击退朝向
      (Variables|Default|SetAttackDirection (Math|Vector|GetForwardVector (Math|Rotator|MakeRotator (.roll (Math|Rotator|MakeRotfromX _output_get_4)) 45.0 (.yaw (Math|Rotator|MakeRotfromX _output_get_4))))) ; 修改朝向
      (Class|AuraAbilitySystemLibrary|SetEffectParamsTargetASC (Variables|Default|GetExplsionDamage%20Params) (Variables|Default|GetTargetAsc))
      (Class|AuraAbilitySystemLibrary|SetKnockbackDirection (Variables|Default|GetExplsionDamage%20Params) (Variables|Default|GetAttackDirection) (Variables|Default|GetKnockback%20Magnitude))
      (Class|AuraAbilitySystemLibrary|SetDeathImpulseDirection (Variables|Default|GetExplsionDamage%20Params) (Variables|Default|GetAttackDirection) (Variables|Default|GetDeathMagnitude))
      (Class|AuraAbilitySystemLibrary|ApplyDamageEffect (Variables|Default|GetExplsionDamage%20Params)))))