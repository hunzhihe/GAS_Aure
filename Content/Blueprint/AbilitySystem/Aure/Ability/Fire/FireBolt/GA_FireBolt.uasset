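; GA_FireBolt is a gameplay ability that casts a fire bolt projectile toward the point under the mouse.
; On activation it commits, gets the cursor hit location from target data and turns the avatar toward it through CombatInterface.
; It plays the cast montage, waits for the Event.Montage.FireBolt gameplay event to spawn the projectile in time with the animation, then ends after a short delay.
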(event Ability|EventActivateAbility
  (Ability|CommitAbility)
  (bind _datahandle (|TargetDataUnderMouse)
    (:ValidData
      (Variables|Default|SetProjectileTargetLocation (.Location (Collision|BreakHitResult (Ability|TargetData|GetHitResultfromTargetData _datahandle))))
      (bind _ascombat_interface (Utilities|Casting|CastToCombatInterface (Ability|GetAvatarActorfromActorInfo)))
      (Class|CombatInterface|UpdateFacingTarget _ascombat_interface (Variables|Default|GetProjectileTargetLocation))
      (|PlayMontageandWaitProxy "None" "/Game/Assets/Characters/Aura/Animations/Abilities/AM_Cast_FireBolt.AM_Cast_FireBolt" 0.8 "None" true 1.0 0.0 false
        (:then
          (Ability|Tasks|WaitGameplayEvent "(TagName=\"Event.Montage.FireBolt\")" 0 true
            (:EventReceived
              (Class|AureProjectSpell|SpawnProjectile (Variables|Default|GetProjectileTargetLocation) (Variables|Default|GetSocket%20Tag) false 0.0)
              (Utilities|FlowControl|Delay 0.5)
              (Ability|EndAbility))))))))

(event Ability|EventOnEndAbility
  (params (bWasCancelled :type Boolean)))